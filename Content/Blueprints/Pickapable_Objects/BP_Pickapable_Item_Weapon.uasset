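; Weapon pickup actor that puts its weapon item into the player's inventory when picked up.
; Its DOIT event calls SetWeapon, which passes Item to the player Inventory's AddWeaponItem, then destroys the actor.
; An unconnected branch in SetWeapon that would snap the weapon to a player not already holding one never runs.
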(event `self.DOIT`
  (`self.Set_Weapon`)
  (`self.K2_DestroyActor`))

(fn `Set_Weapon`
  (`/Game/Blueprints/Inventory/BPC_Inventory.Add_Weapon_Item` (`/Game/Blueprints/CharactersLogic/BP_Player.Inventory` (`self.As BP Player`)) (`self.Item`))
  (return))

(fn `UserConstructionScript`
  (`parent.UserConstructionScript`))