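; Base pickup Blueprint that gives the player either a weapon or souls, chosen by its type enum.
; While the player overlaps its collision, a looping timer polls pick_up until the overlap ends.
; When CanPickUp passes, weapons snap to a player not already holding one, souls add to the player's total and can reset a death count of one, and the pickup destroys itself.
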(event `self.ReceiveBeginPlay`
  (bind _asbp_player (cast `/Game/Blueprints/CharactersLogic/BP_Player` (`GameplayStatics.GetPlayerPawn` 0)))
  (set `self.As BP Player` _asbp_player))

(event `self.Collision.OnComponentBeginOverlap`
  (params (OverlappedComponent :type "PrimitiveComponent Object Reference") (OtherActor :type "Actor Object Reference") (OtherComp :type "PrimitiveComponent Object Reference") (OtherBodyIndex :type Integer) (bFromSweep :type Boolean) (SweepResult :type "HitResult Structure (by ref)"))
  (bind _as_bp_player (`self.As BP Player`))
  (if (== OtherActor _as_bp_player)
    (set `self.Other Actor` OtherActor)
    (set `/Game/Blueprints/CharactersLogic/BP_Player.Is_Overlap?` true _as_bp_player)
    (`KismetSystemLibrary.K2_SetTimer` null "pick_up" 0.1 true)))

(event `pick_up`
  (bind _other_actor (`self.Other Actor`))
  (bind _as_bp_player (`self.As BP Player`))
  (bind _as_bp_player_2 (`self.As BP Player`))
  (bind _as_bp_player_3 (`self.As BP Player`))
  (switch `/Game/Blueprints/Pickapable_Objects/EN_Item_Type` (`self.EN_Type`)
    (:`NewEnumerator0`
      (if (and (`self.Can_Pick_Up?` _other_actor) (not (`/Game/Blueprints/CharactersLogic/BP_Player.Is_Holding?` (`self.As BP Player`))))
        (`/Game/Blueprints/CharactersLogic/BP_Character_Base.Snap_Weapon` _as_bp_player_3 (`self.Item`))
        (set `/Game/Blueprints/CharactersLogic/BP_Player.Is_Holding?` true _as_bp_player_3)
        (`self.K2_DestroyActor`)))
    (:`NewEnumerator2`
      (if (`self.Can_Pick_Up?` _other_actor)
        (set `/Game/Blueprints/CharactersLogic/BP_Character_Base.Souls` (+ (`self.Souls`) (`/Game/Blueprints/CharactersLogic/BP_Character_Base.Souls` _as_bp_player_2)) _as_bp_player_2)
        (if (and (== _other_actor _as_bp_player) (== (`/Game/Blueprints/CharactersLogic/BP_Character_Base.Death_Count` _as_bp_player) 1))
          (set `/Game/Blueprints/CharactersLogic/BP_Character_Base.Death_Count` 0 _as_bp_player))
        (`self.K2_DestroyActor`)))))

(event `self.Collision.OnComponentEndOverlap`
  (params (OverlappedComponent :type "PrimitiveComponent Object Reference") (OtherActor :type "Actor Object Reference") (OtherComp :type "PrimitiveComponent Object Reference") (OtherBodyIndex :type Integer))
  (bind _as_bp_player (`self.As BP Player`))
  (if (== OtherActor _as_bp_player)
    (set `/Game/Blueprints/CharactersLogic/BP_Player.Is_Overlap?` false _as_bp_player)
    (`KismetSystemLibrary.K2_ClearTimer` null "pick_up")))

(fn `UserConstructionScript`)