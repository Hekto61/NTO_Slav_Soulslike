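; BP_Pickapable_Soul is a pickup that grants souls to the player and then removes itself.
; Its DOIT event calls AddSouls, then destroys the actor.
; AddSouls adds the pickup's Souls value to the player's total, then resets the player's DeathCount from one to zero if OtherActor is that player.
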(event `self.DOIT`
  (`self.Add_Souls`)
  (`self.K2_DestroyActor`))

(fn `Add_Souls`
  (bind _as_bp_player (`self.As BP Player`))
  (bind _as_bp_player_2 (`self.As BP Player`))
  (set `/Game/Blueprints/CharactersLogic/BP_Character_Base.Souls` (+ (`self.Souls`) (`/Game/Blueprints/CharactersLogic/BP_Character_Base.Souls` _as_bp_player_2)) _as_bp_player_2)
  (if (and (== (`self.Other Actor`) _as_bp_player) (== (`/Game/Blueprints/CharactersLogic/BP_Character_Base.Death_Count` _as_bp_player) 1))
    (set `/Game/Blueprints/CharactersLogic/BP_Character_Base.Death_Count` 0 _as_bp_player)
    (return)))

(fn `UserConstructionScript`
  (`parent.UserConstructionScript`))