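; Base enemy Blueprint that equips a weapon on spawn and rewards the player with souls on death.
; BeginPlay snaps the weapon class and caches the player pawn as BP_Player.
; Death adds the enemy's Souls to that player, then destroys the enemy and its current weapon.
; CalculateDamage passes to the parent only when the instigator is BP_Player, while the hit event is overridden empty.
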(event `self.ReceiveBeginPlay`
  (`parent.ReceiveBeginPlay`)
  (`self.Snap_Weapon` (`self.Weapon_Class`))
  (bind _asbp_player (cast `/Game/Blueprints/CharactersLogic/BP_Player` (`GameplayStatics.GetPlayerPawn` 0)))
  (set `self.As BP Player` _asbp_player))

(event `self.Event_On_Death`
  (bind _as_bp_player (`self.As BP Player`))
  (set `/Game/Blueprints/CharactersLogic/BP_Character_Base.Souls` (+ (`self.Souls`) (`/Game/Blueprints/CharactersLogic/BP_Character_Base.Souls` _as_bp_player)) _as_bp_player)
  (`self.K2_DestroyActor`)
  (`self.K2_DestroyActor` (`self.Current_Weapon`)))

(event `self.Event_On_Hit`
  (params (instigator :type "Actor Object Reference")))

(fn `Calculate_Damage`
  (params (Bone_Name :type Name) (Damage :type "Float (double-precision)") (Instigator :type "Actor Object Reference"))
  (cast `/Game/Blueprints/CharactersLogic/BP_Player` Instigator)
  (`parent.Calculate_Damage` Bone_Name Damage Instigator))

(fn `UserConstructionScript`
  (`parent.UserConstructionScript`))