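; Baba Yaga boss AI character that focuses on the player, curses them and teleports when hit.
; Entering the Curse sphere starts a looping timer that adds curse stacks and applies cursed speed, spawning a cone target and curse-clear actor if the player is uncursed.
; Hits trigger a jump to a random navigable point, gated by a delayed cooldown flag.
; Short and long range overlaps are empty, and the timer clear is unconnected.
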(event `self.ReceiveBeginPlay`
  (`parent.ReceiveBeginPlay`)
  (`AIController.K2_SetFocus` (`AIBlueprintHelperLibrary.GetAIController` self) (`self.As BP Player`)))

(event `self.Short_Range.OnComponentBeginOverlap`
  (params (OverlappedComponent :type "PrimitiveComponent Object Reference") (OtherActor :type "Actor Object Reference") (OtherComp :type "PrimitiveComponent Object Reference") (OtherBodyIndex :type Integer) (bFromSweep :type Boolean) (SweepResult :type "HitResult Structure (by ref)"))
  ;[1 1 1] Short_range
)

(event `self.Short_Range.OnComponentEndOverlap`
  (params (OverlappedComponent :type "PrimitiveComponent Object Reference") (OtherActor :type "Actor Object Reference") (OtherComp :type "PrimitiveComponent Object Reference") (OtherBodyIndex :type Integer))
  ;[1 1 1] Short_range
)

(event `self.Long_Range.OnComponentBeginOverlap`
  (params (OverlappedComponent :type "PrimitiveComponent Object Reference") (OtherActor :type "Actor Object Reference") (OtherComp :type "PrimitiveComponent Object Reference") (OtherBodyIndex :type Integer) (bFromSweep :type Boolean) (SweepResult :type "HitResult Structure (by ref)"))
  ;[1 1 1] Long_Ranhge
)

(event `self.Long_Range.OnComponentEndOverlap`
  (params (OverlappedComponent :type "PrimitiveComponent Object Reference") (OtherActor :type "Actor Object Reference") (OtherComp :type "PrimitiveComponent Object Reference") (OtherBodyIndex :type Integer))
  ;[1 1 1] Long_Ranhge
)

(event `self.Curse.OnComponentBeginOverlap`
  (params (OverlappedComponent :type "PrimitiveComponent Object Reference") (OtherActor :type "Actor Object Reference") (OtherComp :type "PrimitiveComponent Object Reference") (OtherBodyIndex :type Integer) (bFromSweep :type Boolean) (SweepResult :type "HitResult Structure (by ref)"))
  (bind _as_bp_player (`self.As BP Player`))
  ;[1 1 1] Curse
  (if (== OtherActor _as_bp_player)
    (if (`/Game/Blueprints/CharactersLogic/BP_Player.Is_Cursed?` _as_bp_player)
      (`KismetSystemLibrary.K2_SetTimer` null "Start_Curse" 5.0 true)
      (else
        (`self.Start_Curse`)
        (`|SpawnActorFromClass` "/Game/Blueprints/AI/Boss_AI/BP_Cone_Target.BP_Cone_Target_C" (`KismetMathLibrary.MakeTransform` (+ (* (`self.GetActorForwardVector`) -1000.0) (`self.K2_GetActorLocation`))) "Undefined" "OverrideRootScale" null null)
        (`|SpawnActorFromClass` "/Game/Blueprints/AI/Boss_AI/BP_Clear_Curse_BY.BP_Clear_Curse_BY_C" (`KismetMathLibrary.MakeTransform` (`NavigationSystemV1.K2_GetRandomReachablePointInRadius` (`self.K2_GetActorLocation`) (`SphereComponent.SphereRadius` (`self.Curse`)) null null)) "Undefined" "OverrideRootScale" null null)
        (`KismetSystemLibrary.K2_SetTimer` null "Start_Curse" 5.0 true)))))

(event `self.Curse.OnComponentEndOverlap`
  (params (OverlappedComponent :type "PrimitiveComponent Object Reference") (OtherActor :type "Actor Object Reference") (OtherComp :type "PrimitiveComponent Object Reference") (OtherBodyIndex :type Integer))
  ;[1 1 1] Curse
  (if (== OtherActor (`self.As BP Player`))
    _))

(event `Start_Curse`
  (bind _as_bp_player (`self.As BP Player`))
  (`/Engine/EditorBlueprintResources/StandardMacros.IncrementFloat` (`/Game/Blueprints/CharactersLogic/BP_Player.Stack` _as_bp_player)
    (:`  `
      (set `/Game/Blueprints/CharactersLogic/BP_Player.Is_Cursed?` true _as_bp_player)
      (`/Game/Blueprints/CharactersLogic/BP_Player.Cursed_Speed` _as_bp_player))))

(event `/Game/Blueprints/CharactersLogic/BP_Character_Base.Event_On_Hit`
  (bind _randomlocation (`NavigationSystemV1.K2_GetRandomLocationInNavigableRadius` (`self.K2_GetActorLocation`) (`SphereComponent.SphereRadius` (`self.Curse`)) null null))
  (if (`self.Teleport_Delay`)
    (`KismetSystemLibrary.Delay` 20.0)
    (set `self.Teleport_Delay` false)
    (else
      (bind (_sweephitresult _returnvalue) (`self.K2_SetActorLocation` (`KismetMathLibrary.MakeVector` (.x _randomlocation) (.y _randomlocation) (+ (.z _randomlocation) 100.0)) false true))
      (set `self.Teleport_Delay` true))))

(fn `UserConstructionScript`
  (`parent.UserConstructionScript`))