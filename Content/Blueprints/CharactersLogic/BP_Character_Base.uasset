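; Base character Blueprint handling health, stamina, sprinting, melee attacks and mead healing, with empty hit and death events.
; Timers drive sprint drain and stamina regen; montage-length delays gate attacks and drinking, and NPCs skip attack stamina cost.
; Damage from others lowers health, and death releases the player's target lock.
; Weapons spawn onto a hand socket and supply attack montage and cost, while body parts follow the main mesh via master pose.
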(event `Event_On_Death`)

(event `Event_On_Hit`
  (params (instigator :type "Actor Object Reference")))

(event `Event_Restore_Health`
  (params (`Is_Reastore?` :type Boolean))
  (set `self.Is Reastore?` `Is_Reastore?`)
  (if (and (and (< (`self.Health_Current`) (`self.Health_Max`)) (> (`self.Mead_Count`) 0) (> (`self.Health_Current`) 0.0)) (`self.Is Reastore?`) (not (`self.Restore_Delay`)))
    (set `self.Restore_Delay` true)
    (`/Engine/EditorBlueprintResources/StandardMacros.IsValid` (`self.Current_Weapon`)
      (:`Is Valid`
        (`self.SetActorHiddenInGame` (`self.Current_Weapon`) true))
      (:`Is Not Valid`
        _))
    (`SceneComponent.SetHiddenInGame` (`self.mead`) false true)
    (bind _returnvalue (`self.PlayAnimMontage` "/Game/Resourse/Character_Mine/Anims/man_skel_drink_Drink_Montage.man_skel_drink_Drink_Montage"))
    (`KismetSystemLibrary.Delay` _returnvalue)
    (`self.Health Reastore`)
    (`SceneComponent.SetHiddenInGame` (`self.mead`) true true)
    (`/Engine/EditorBlueprintResources/StandardMacros.IsValid` (`self.Current_Weapon`)
      (:`Is Valid`
        (`self.SetActorHiddenInGame` (`self.Current_Weapon`) false))
      (:`Is Not Valid`
        _))
    (set `self.Restore_Delay` false)))

(event `Set_Weapon_Master`
  (bind _asbp_weapon_base (cast `/Game/Blueprints/WeaponLogic/BP_Weapon_Base` (`self.Current_Weapon`)))
  (set `self.Weapon_Master_Ref` _asbp_weapon_base))

(event `self.ReceiveBeginPlay`
  (`self.Set_Health`))

(event `/Game/Blueprints/WeaponLogic/Interfaces/BPI_Take_Damage.Taking_Damage`
  (params (Bone_Name :type Name) (Damage :type "Float (double-precision)") (Instigator :type "Actor Object Reference"))
  (`self.Event_On_Hit` Instigator)
  (if (!= Instigator (`self.GetOwner`))
    (`self.Calculate_Damage` Bone_Name Damage Instigator)))

(event `Event_Attack`
  (params (`Is_Attack?` :type Boolean))
  (set `self.Is_Attack?` `Is_Attack?`)
  (if (`self.can attack?`)
    (set `self.Attacking_Delay` true)
    (bind _returnvalue (`self.PlayAnimMontage` (`/Game/Blueprints/WeaponLogic/BP_Weapon_Base.Attack Montage` (`self.Weapon_Master_Ref`))))
    (`KismetSystemLibrary.RetriggerableDelay` _returnvalue)
    (if (not (`self.Is_NPC?`))
      (`self.Stamina_Drain_Attack`))
    (set `self.Attacking_Delay` false)
    (else
      (`KismetSystemLibrary.K2_ClearTimer` null "Stamina_Restore"))))

(event `Sprint`
  (params (`Sprint?` :type Boolean))
  (bind _charactermovement (`self.CharacterMovement`))
  ;[0.05098 0.05098 0.05098] Sprint
  (if (and `Sprint?` (!= (`KismetMathLibrary.VSize` (`self.GetVelocity`)) 0.0))
    (if (>= (`self.Stamina_Current`) (`self.Stamina_Sprint_Cost`))
      (set `CharacterMovementComponent.MaxWalkSpeed` (* (`self.Running_Speed_Mult`) (`self.Current_Speed`)) _charactermovement)
      (bind _output_get (set `self.Is_Sprinting?` true))
      (`KismetSystemLibrary.K2_SetTimer` null "Stamina_Drain_Sprint" 0.5 _output_get))
    (else
      (set `CharacterMovementComponent.MaxWalkSpeed` (`self.Current_Speed`) _charactermovement)
      (`KismetSystemLibrary.K2_SetTimer` null "Stamina_Restore" 0.5 true)
      (`KismetSystemLibrary.K2_ClearTimer` null "Stamina_Drain_Sprint")
      (set `self.Is_Sprinting?` false))))

(event `Stamina_Drain_Sprint`
  (bind _stamina_current (`self.Stamina_Current`))
  (bind _stamina_sprint_cost (`self.Stamina_Sprint_Cost`))
  ;[0.05098 0.05098 0.05098] Sprint
  (set `self.Stamina_Current` (`KismetMathLibrary.FMax` (- _stamina_current _stamina_sprint_cost)))
  (if (not (and (>= _stamina_current _stamina_sprint_cost) (!= (`KismetMathLibrary.VSize` (`self.GetVelocity`)) 0.0)))
    (set `CharacterMovementComponent.MaxWalkSpeed` (`self.Current_Speed`) (`self.CharacterMovement`))
    (`KismetSystemLibrary.K2_ClearTimer` null "Stamina_Drain_Sprint")
    (set `self.Is_Sprinting?` false)))

(event `Stamina_Restore`
  ;[0.05098 0.05098 0.05098] Sprint
  (if (and (< (`self.Stamina_Current`) (`self.Stamina_Max`)) (not (`self.Is_Sprinting?`)))
    (set `self.Stamina_Current` (+ (`self.Stamina_Current`) (`self.Stamina_Recharge_Rate`)))
    (else
      (`KismetSystemLibrary.K2_ClearTimer` null "Stamina_Restore"))))

(event `Stamina_Drain_Attack`
  (bind _stamina_current (`self.Stamina_Current`))
  ;[0.05098 0.05098 0.05098] Sprint
  (set `self.Stamina_Current` (`KismetMathLibrary.FMax` (- _stamina_current (`/Game/Blueprints/WeaponLogic/BP_Weapon_Base.Stamina Cost` (`self.Weapon_Master_Ref`)))))
  (if (>= _stamina_current 0.0)
    (`KismetSystemLibrary.K2_SetTimer` null "Stamina_Restore" 0.5 true)
    (else
      (`KismetSystemLibrary.K2_ClearTimer` null "Stamina_Restore"))))

(fn `Calculate_Damage`
  (params (Bone_Name :type Name) (Damage :type "Float (double-precision)") (Instigator :type "Actor Object Reference"))
  (locals (Damage_Loc :type "Float (double-precision)"))
  (set `local.Damage_Loc` Damage)
  (set `self.Health_Current` (- (`self.Health_Current`) (`local.Damage_Loc`)))
  (`self.Death`))

(fn `Death`
  (if (<= (`self.Health_Current`) 0.0)
    (`|ExecutionSequence`
      (:`then_0`
        (`self.Event_On_Death`))
      (:`then_1`
        (bind _asbp_player (cast `/Game/Blueprints/CharactersLogic/BP_Player` (`GameplayStatics.GetPlayerPawn` 0)))
        (`TargetSystemComponent.TargetLockOff` (`/Game/Blueprints/CharactersLogic/BP_Player.TargetSystem` _asbp_player))))))

(fn `Health Reastore`
  (`/Engine/EditorBlueprintResources/StandardMacros.DecrementInt` (`self.Mead_Count`)
    (:`  `
      (set `self.Health_Current` (+ (* (/ (`self.Health_Max`) 100.0) 50.0) (`self.Health_Current`)))
      (if (> (`self.Health_Current`) (`self.Health_Max`))
        (set `self.Health_Current` (`self.Health_Max`))))))

(fn `Set_Health`
  (set `self.Health_Current` (`self.Health_Max`))
  (set `self.Stamina_Current` (`self.Stamina_Max`))
  (bind _output_get (set `self.Current_Speed` (`self.Default_Speed`)))
  (set `CharacterMovementComponent.MaxWalkSpeed` _output_get (`self.CharacterMovement`))
  (set `self.Mead_Count` 3))

(fn `Snap_Weapon`
  (params (Class :type "Actor Class Reference"))
  (bind _mesh (`self.Mesh`))
  (bind _returnvalue (`|SpawnActorFromClass` Class (`SceneComponent.GetSocketTransform` _mesh "SKT_weapon_R" "RTS_World") "Undefined" "OverrideRootScale" self null))
  (bind _output_get (set `self.Weapon` _returnvalue))
  (`self.K2_AttachToComponent` _output_get _mesh (`SkinnedMeshComponent.GetSocketBoneName` _mesh "SKT_weapon_R") "KeepWorld" "KeepWorld" "KeepWorld" true)
  (set `self.Current_Weapon` (`self.Weapon`))
  (`self.Set_Weapon_Master`))

(fn `UserConstructionScript`
  (`SceneComponent.K2_AttachToComponent` (`self.mead`) (`self.Mesh`) "SKT_weapon_R" "KeepRelative" "KeepRelative" "KeepRelative" true)
  (`SkinnedMeshComponent.SetLeaderPoseComponent` (`self.Legs`) (`self.Mesh`) false)
  (`SkinnedMeshComponent.SetLeaderPoseComponent` (`self.Arms`) (`self.Mesh`) false)
  (`SkinnedMeshComponent.SetLeaderPoseComponent` (`self.Head`) (`self.Mesh`) false))