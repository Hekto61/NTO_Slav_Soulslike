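; Inventory component that stores collected weapons and armor and handles equipping them on the player.
; Add events append items to separate weapon and armor collections, while equipped armor is stored in a map keyed by armor type.
; Equipping casts player character 0 to BP_Player: armor triggers a stat refresh, while weapons destroy the current weapon actor, snap on the new one and set the holding flag.
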(event `Add_Weapon_Item`
  (params (New_Weapon :type "Actor Class Reference (by ref)"))
  (`KismetArrayLibrary.Array_Add` (`self.Weapon_Inveentory`) New_Weapon))

(event `Add_Armor_Item`
  (params (new_armor :type "/Game/Blueprints/Armour_Logic/Armor_Data/ST_Armor_Details Structure"))
  (`KismetArrayLibrary.Array_Add` (`self.Armor_Inventory`) new_armor))

(event `Equip_Armour`
  (params (`Armour Type` :type "/Game/Blueprints/Armour_Logic/Armor_Data/EN_Armour_Type Enum" :default "NewEnumerator0") (Armour :type "/Game/Blueprints/Armour_Logic/Armor_Data/ST_Armor_Details Structure"))
  (`BlueprintMapLibrary.Map_Add` (`self.Equipped_Armor`) `Armour Type` Armour)
  (bind _asbp_player (cast `/Game/Blueprints/CharactersLogic/BP_Player` (`GameplayStatics.GetPlayerCharacter` 0)))
  (`/Game/Blueprints/CharactersLogic/BP_Player.Refresh_Stats` _asbp_player))

(event `Equip_Weqpon`
  (params (NewParam :type "Actor Class Reference"))
  (bind _asbp_player (cast `/Game/Blueprints/CharactersLogic/BP_Player` (`GameplayStatics.GetPlayerCharacter` 0)))
  (`Actor.K2_DestroyActor` (`/Game/Blueprints/CharactersLogic/BP_Character_Base.Current_Weapon` _asbp_player))
  (`/Game/Blueprints/CharactersLogic/BP_Character_Base.Snap_Weapon` _asbp_player NewParam)
  (set `/Game/Blueprints/CharactersLogic/BP_Player.Is_Holding?` true _asbp_player))