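; AI controller Blueprint that drives a pawn with the BT_NEW_Main behavior tree.
; On possess it starts the tree and calls SetMasterCharRef, whose event casts the controlled pawn to BP_Character_Base and caches it.
; Perception updates write whether the stimulus was sensed into the Can_See_Player? blackboard key, without checking which actor was perceived.
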(event `Set_Master_Char_Ref`
  (bind _asbp_character_base (cast `/Game/Blueprints/CharactersLogic/BP_Character_Base` (`self.K2_GetPawn`)))
  (set `self.Master_Ref_Character_Base` _asbp_character_base))

(event `self.ReceiveBeginPlay`)

(event `self.ReceivePossess`
  (params (PossessedPawn :type "Pawn Object Reference"))
  (`self.RunBehaviorTree` "/Game/Blueprints/AI/BT_NEW_Main.BT_NEW_Main")
  (`self.Set_Master_Char_Ref`))

(event `self.AIPerception.OnTargetPerceptionUpdated`
  (params (Actor :type "Actor Object Reference") (Stimulus :type "AIStimulus Structure"))
  (`BlackboardComponent.SetValueAsBool` (`AIBlueprintHelperLibrary.GetBlackboard` null) "Can_See_Player?" (`.bSuccessfullySensed` (break `AIStimulus` Stimulus))))

(fn `UserConstructionScript`)