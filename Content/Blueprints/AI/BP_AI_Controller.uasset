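; AI controller that drives a BP_Character_Base pawn through the BT_Main behavior tree.
; On possess it starts the tree, caches the controlled character, stores player pawn 0 as its current target and writes its state to the EN_AI_State blackboard key.
; AI_Attack changes that state and updates the blackboard, while Attack forwards its flag to the character's EventAttack.
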(event `Set_Master_Char_Ref`
  (bind _asbp_character_base (cast `/Game/Blueprints/CharactersLogic/BP_Character_Base` (`self.K2_GetPawn`)))
  (set `self.Master_Ref_Character_Base` _asbp_character_base))

(event `self.ReceiveBeginPlay`)

(event `self.ReceivePossess`
  (params (PossessedPawn :type "Pawn Object Reference"))
  (`self.RunBehaviorTree` "/Game/Blueprints/AI/BT_Main.BT_Main")
  (`self.Set_Master_Char_Ref`)
  (set `self.Current_Target` (`GameplayStatics.GetPlayerPawn` 0))
  (`BlackboardComponent.SetValueAsEnum` (`AIBlueprintHelperLibrary.GetBlackboard` null) "EN_AI_State" (`self.Current_State`)))

(event `AI_Attack`
  (bind _output_get (set `self.Current_State` "NewEnumerator1"))
  (`BlackboardComponent.SetValueAsEnum` (`AIBlueprintHelperLibrary.GetBlackboard` null) "EN_AI_State" _output_get))

(event `Attack`
  (params (`Is_Attack?` :type Boolean))
  (`/Game/Blueprints/CharactersLogic/BP_Character_Base.Event_Attack` (`self.Master_Ref_Character_Base`) `Is_Attack?`))

(fn `UserConstructionScript`)