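; BP_Cone_Target is a cone target in the boss AI folder that is destroyed when the player damages it.
; On BeginPlay it caches the BP_Player pawn and starts a looping timer that polls the player's Stack value.
; The timer toggles custom depth rendering on the cone, turning it on while Stack is at or below a fixed threshold.
; TakingDamage destroys the actor only when the instigator is that cached player, regardless of damage amount.
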(event `self.ReceiveBeginPlay`
  (bind _asbp_player (cast `/Game/Blueprints/CharactersLogic/BP_Player` (`GameplayStatics.GetPlayerPawn` 0)))
  (set `self.As BP Player` _asbp_player)
  (`KismetSystemLibrary.K2_SetTimer` null "Outline" 0.1 true))

(event `Outline`
  (if (<= (`/Game/Blueprints/CharactersLogic/BP_Player.Stack` (`self.As BP Player`)) 3.0)
    (`PrimitiveComponent.SetRenderCustomDepth` (`self.Cone`) true)
    (else
      (`PrimitiveComponent.SetRenderCustomDepth` (`self.Cone`) false))))

(event `/Game/Blueprints/WeaponLogic/Interfaces/BPI_Take_Damage.Taking_Damage`
  (params (Bone_Name :type Name) (Damage :type "Float (double-precision)") (Instigator :type "Actor Object Reference"))
  (if (== Instigator (`self.As BP Player`))
    (`self.K2_DestroyActor`)))

(fn `UserConstructionScript`)