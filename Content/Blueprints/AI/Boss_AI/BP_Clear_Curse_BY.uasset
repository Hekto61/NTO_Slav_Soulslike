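; Interactable pickup in the Baba Yaga boss fight that lifts the curse from the player.
; A looping timer toggles the cylinder's custom depth outline based on the player's Stack value.
; Sphere overlap starts a polling timer that waits for E held while the player is cursed and no BP_Cone_Target actors remain.
; It then clears the player's cursed speed, stops the boss's curse timer, resets its sphere and destroys itself.
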(event `self.ReceiveBeginPlay`
  (bind _asbp_player (cast `/Game/Blueprints/CharactersLogic/BP_Player` (`GameplayStatics.GetPlayerPawn` 0)))
  (set `self.As BP Player` _asbp_player)
  (`KismetSystemLibrary.K2_SetTimer` null "Outline" 0.1 true))

(event `Outline`
  (if (<= (`/Game/Blueprints/CharactersLogic/BP_Player.Stack` (`self.As BP Player`)) 3.0)
    (`PrimitiveComponent.SetRenderCustomDepth` (`self.Cylinder`) true)
    (else
      (`PrimitiveComponent.SetRenderCustomDepth` (`self.Cylinder`) false))))

(event `self.Sphere.OnComponentBeginOverlap`
  (params (OverlappedComponent :type "PrimitiveComponent Object Reference") (OtherActor :type "Actor Object Reference") (OtherComp :type "PrimitiveComponent Object Reference") (OtherBodyIndex :type Integer) (bFromSweep :type Boolean) (SweepResult :type "HitResult Structure (by ref)"))
  (bind _as_bp_player (`self.As BP Player`))
  (if (== OtherActor _as_bp_player)
    (set `self.Other Actor` OtherActor)
    (set `/Game/Blueprints/CharactersLogic/BP_Player.Is_Overlap?` true _as_bp_player)
    (`KismetSystemLibrary.K2_SetTimer` null "Interuct" 0.1 true)))

(event `self.Sphere.OnComponentEndOverlap`
  (params (OverlappedComponent :type "PrimitiveComponent Object Reference") (OtherActor :type "Actor Object Reference") (OtherComp :type "PrimitiveComponent Object Reference") (OtherBodyIndex :type Integer))
  (bind _as_bp_player (`self.As BP Player`))
  (if (== OtherActor _as_bp_player)
    (set `/Game/Blueprints/CharactersLogic/BP_Player.Is_Overlap?` false _as_bp_player)
    (`KismetSystemLibrary.K2_ClearTimer` null "Interuct")))

(event `Interuct`
  (bind _as_bp_player (`self.As BP Player`))
  (bind _outactors (`GameplayStatics.GetAllActorsOfClass` "/Game/Blueprints/AI/Boss_AI/BP_Cone_Target.BP_Cone_Target_C"))
  (if (and (== (`self.Other Actor`) _as_bp_player) (`PlayerController.IsInputKeyDown` (`GameplayStatics.GetPlayerController` 0) "E") (`/Game/Blueprints/CharactersLogic/BP_Player.Is_Cursed?` _as_bp_player) (== (`KismetArrayLibrary.Array_Length` _outactors) 0))
    (`/Game/Blueprints/CharactersLogic/BP_Player.Clear_Cursed_Speed` (`self.As BP Player`))
    (bind _returnvalue (`GameplayStatics.GetActorOfClass` "/Game/Blueprints/CharactersLogic/BP_AI_BOSS_Baba_Yaga.BP_AI_BOSS_Baba_Yaga_C"))
    (`/Engine/EditorBlueprintResources/StandardMacros.IsValid` _returnvalue
      (:`Is Valid`
        (`KismetSystemLibrary.K2_ClearTimer` _returnvalue "Start_Curse")
        (`/Game/Blueprints/CharactersLogic/BP_AI_BOSS_Baba_Yaga.Reset_Sphere` _returnvalue true))
      (:`Is Not Valid`
        _))
    (`self.K2_DestroyActor`)))

(fn `UserConstructionScript`)