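; Boss AI projectile that can home in on the player, damaging it on impact through a TakingDamage message.
; BeginPlay caches the player pawn, and the Lock_on event makes one of its scene components the ProjectileMovement homing target.
; Any hit spawns a water-ball particle effect and destroys the projectile.
; A closest-player search function and a repeating lock-on loop exist but are never run.
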(event `self.ReceiveBeginPlay`
  (bind _asbp_player (cast `/Game/Blueprints/CharactersLogic/BP_Player` (`GameplayStatics.GetPlayerPawn` 0)))
  (set `self.As BP Player` _asbp_player))

(event `Lock_on`
  (bind _projectilemovement (`self.ProjectileMovement`))
  (set `ProjectileMovementComponent.HomingTargetComponent` (`self.GetComponentByClass` (`self.As BP Player`) "/Script/Engine.SceneComponent") _projectilemovement)
  (set `ProjectileMovementComponent.bIsHomingProjectile` true _projectilemovement))

(event `self.ReceiveHit`
  (params (MyComp :type "PrimitiveComponent Object Reference") (Other :type "Actor Object Reference") (OtherComp :type "PrimitiveComponent Object Reference") (bSelfMoved :type Boolean) (HitLocation :type "Vector Structure") (HitNormal :type "Vector Structure") (NormalImpulse :type "Vector Structure") (Hit :type "HitResult Structure (by ref)"))
  (cast `/Game/Blueprints/CharactersLogic/BP_Player` Other
    (:`then`
      (message `/Game/Blueprints/WeaponLogic/Interfaces/BPI_Take_Damage.Taking_Damage` Other "None" 10.0 (`self.GetOwner`)))
    (:`CastFailed`
      _))
  (`GameplayStatics.SpawnEmitterAtLocation` "/Game/FXVarietyPack/Particles/P_ky_waterBallHit.P_ky_waterBallHit" HitLocation)
  (`self.K2_DestroyActor`))

(fn `Find_Homing_Target`
  (returns (Target :type "SceneComponent Object Reference"))
  (bind _outactors (`GameplayStatics.GetAllActorsOfClass` "/Game/Blueprints/CharactersLogic/BP_Player.BP_Player_C"))
  (for _array_element _outactors
    (bind _returnvalue (`KismetMathLibrary.VSize` (- (`self.K2_GetActorLocation` _array_element) (`self.K2_GetActorLocation`))))
    (if (< _returnvalue (`self.Closest_Target`))
      (set `self.Closest_Target` _returnvalue)
      (set `self.Target` _array_element)))
  (return (`self.GetComponentByClass` (`self.Target`) "/Script/Engine.SceneComponent")))

(fn `UserConstructionScript`)