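; AI spawner actor that fills the level with AI of a configurable class, passing each health, weapon class and souls values.
; On BeginPlay it caches the player, then starts a fast looping timer that spawns at its own location until the world-wide count of that class reaches Count, then clears itself.
; A destroy-all event removes every actor of that class and its current weapon.
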(event `self.ReceiveBeginPlay`
  (bind _asbp_player (cast `/Game/Blueprints/CharactersLogic/BP_Player` (`GameplayStatics.GetPlayerPawn` 0)))
  (set `self.As BP Player` _asbp_player)
  (`self.Set_Timer`))

(event `Set_Timer`
  (`KismetSystemLibrary.K2_SetTimer` null "Event_Spawn" 0.1 true))

(event `self.ReceiveTick`
  (params (DeltaSeconds :type "Float (single-precision)")))

(event `Event_Spawn`
  (bind _outactors (`GameplayStatics.GetAllActorsOfClass` (`self.Actor Class`)))
  (bind _returnvalue (`KismetArrayLibrary.Array_Length` _outactors))
  (if (and (>= _returnvalue 0) (< _returnvalue (`self.Count`)))
    (`|SpawnActorFromClass` (`self.Actor Class`) (`KismetMathLibrary.MakeTransform` (`self.K2_GetActorLocation`)) "Undefined" "OverrideRootScale" null (`self.Health Max`) (`self.Weapon Class`) (`self.Souls`) null)
    (else
      (`KismetSystemLibrary.K2_ClearTimer` null "Event_Spawn"))))

(event `Event_Destroy_All`
  (bind _outactors (`GameplayStatics.GetAllActorsOfClass` (`self.Actor Class`)))
  (for _array_element _outactors
    (`self.K2_DestroyActor` (`/Game/Blueprints/CharactersLogic/BP_Character_Base.Current_Weapon` _array_element))
    (`self.K2_DestroyActor` _array_element)))

(fn `UserConstructionScript`)