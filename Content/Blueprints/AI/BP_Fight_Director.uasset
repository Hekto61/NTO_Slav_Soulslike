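; BP_Fight_Director is an AI combat director that periodically picks one enemy to attack.
; Set_Director seeds a map of actors with random priority scores and starts a looping attack timer.
; Each tick of that timer scales EnemyList scores by how opposed each enemy's facing is to the camera's forward vector.
; The top scorer's BP_AI_Controller then runs AIAttack, and its score is re-randomized.
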(event `Set_Director`
  (bind _outactors (`GameplayStatics.GetAllActorsOfClass` (`self.Actor Class`)))
  (for _array_element _outactors
    (`BlueprintMapLibrary.Map_Add` (`self.Enemy_Grading`) _array_element (`KismetMathLibrary.RandomFloatInRange` 1.0 5.0)))
  (`KismetSystemLibrary.K2_SetTimerDelegate` (delegate `Trigger_Attack`) 4.0 true))

(event `self.ReceiveBeginPlay`)

(event `Trigger_Attack`
  (`self.Recalculate_Score`)
  (bind (_loc_highest_value1 _loc_highest_great_ai1) (`self.FInd_Highest_Priority`))
  (bind _asbp_ai_controller (cast `/Game/Blueprints/AI/BP_AI_Controller` (`AIBlueprintHelperLibrary.GetAIController` _loc_highest_great_ai1)))
  (`/Game/Blueprints/AI/BP_AI_Controller.AI_Attack` _asbp_ai_controller)
  (`BlueprintMapLibrary.Map_Add` (`self.Enemy_Grading`) _loc_highest_great_ai1 (`KismetMathLibrary.RandomFloatInRange` 1.0 5.0)))

(fn `FInd_Highest_Priority`
  (returns (Loc_Highest_Value1 :type "Float (double-precision)") (Loc_Highest_Great_AI1 :type "/Game/Blueprints/CharactersLogic/BP_enemy_Base Object Reference"))
  (locals (Loc_Highest_Value :type "Float (double-precision)") (Loc_Highest_Great_AI :type "/Game/Blueprints/CharactersLogic/BP_enemy_Base Object Reference"))
  (bind _keys (`BlueprintMapLibrary.Map_Keys` (`self.Enemy_Grading`)))
  (for _array_element _keys
    (bind _value (`BlueprintMapLibrary.Map_Find` (`self.Enemy_Grading`) _array_element))
    (if (> _value (`local.Loc_Highest_Value`))
      (set `local.Loc_Highest_Value` _value)
      (set `local.Loc_Highest_Great_AI` _array_element)))
  (return (`local.Loc_Highest_Value`) (`local.Loc_Highest_Great_AI`)))

(fn `Recalculate_Score`
  (`self.Score_By_Position`))

(fn `Score_By_Position`
  (bind _enemy_grading (`self.Enemy_Grading`))
  (for _array_element (`self.Enemy_List`)
    (`BlueprintMapLibrary.Map_Add` _enemy_grading _array_element (* (`BlueprintMapLibrary.Map_Find` _enemy_grading _array_element) (+ (`KismetMathLibrary.NormalizeToRange` (* (`KismetMathLibrary.Dot_VectorVector` (`self.GetActorForwardVector` _array_element) (`KismetMathLibrary.GetForwardVector` (`PlayerCameraManager.GetCameraRotation` (`GameplayStatics.GetPlayerCameraManager` 0)))) -1.0) -1.0 1.0) 0.5)))))

(fn `UserConstructionScript`)