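; BP_BoneFire is a bonfire checkpoint that saves the player's current location as their last bonfire location.
; While the player overlaps its collision, a looping timer polls the Check graph, which holds a test for the E key and non-activated state.
; Saving reveals the initially hidden particles, activates the audio and marks the bonfire activated.
; The player's IsOverlap flag tracks overlap with an unlit bonfire.
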(event `self.ReceiveBeginPlay`
  (bind _asbp_player (cast `/Game/Blueprints/CharactersLogic/BP_Player` (`GameplayStatics.GetPlayerPawn` 0)))
  (set `self.As BP Player` _asbp_player)
  (`SceneComponent.SetVisibility` (`self.ParticleSystem`) false false))

(event `Save_Bone_Fire_Location`
  (bind _as_bp_player (`self.As BP Player`))
  (if (`self.Check` (`self.Other Actor`))
    (set `/Game/Blueprints/CharactersLogic/BP_Player.Last_BoneFire_Location` (`self.K2_GetActorLocation` _as_bp_player) _as_bp_player)
    (`SceneComponent.SetVisibility` (`self.ParticleSystem`) true false)
    (set `self.Is_Activated?` true)
    (set `/Game/Blueprints/CharactersLogic/BP_Player.Is_Overlap?` false (`self.As BP Player`))
    (`ActorComponent.Activate` (`self.AudioCurveSource`) false)))

(event `self.Collision.OnComponentBeginOverlap`
  (params (OverlappedComponent :type "PrimitiveComponent Object Reference") (OtherActor :type "Actor Object Reference") (OtherComp :type "PrimitiveComponent Object Reference") (OtherBodyIndex :type Integer) (bFromSweep :type Boolean) (SweepResult :type "HitResult Structure (by ref)"))
  (bind _as_bp_player (`self.As BP Player`))
  (if (== OtherActor _as_bp_player)
    (set `self.Other Actor` OtherActor)
    (`KismetSystemLibrary.K2_SetTimer` null "Save_Bone_Fire_Location" 0.1 true)
    (if (not (`self.Is_Activated?`))
      (set `/Game/Blueprints/CharactersLogic/BP_Player.Is_Overlap?` true _as_bp_player))))

(event `self.Collision.OnComponentEndOverlap`
  (params (OverlappedComponent :type "PrimitiveComponent Object Reference") (OtherActor :type "Actor Object Reference") (OtherComp :type "PrimitiveComponent Object Reference") (OtherBodyIndex :type Integer))
  (bind _as_bp_player (`self.As BP Player`))
  (if (== OtherActor _as_bp_player)
    (`KismetSystemLibrary.K2_ClearTimer` null "Save_Bone_Fire_Location")
    (set `/Game/Blueprints/CharactersLogic/BP_Player.Is_Overlap?` false _as_bp_player)))

(fn `UserConstructionScript`)