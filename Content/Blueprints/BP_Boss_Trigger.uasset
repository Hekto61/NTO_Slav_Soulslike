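; BP_Boss_Trigger is a trigger that starts the Baba Yaga boss encounter when the player overlaps it.
; It teleports the player to an arrow marker, turns the hidden cube into a visible blocking barrier, and spawns the boss with preset health, weapon and souls.
; Reset hides the cube, disables its collision, and destroys the boss and its weapon.
; The construction script positions the arrow and scales the cube from per-instance variables.
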(event `self.ReceiveBeginPlay`
  (`SceneComponent.SetHiddenInGame` (`self.Cube`) true false)
  (bind _asbp_player (cast `/Game/Blueprints/CharactersLogic/BP_Player` (`GameplayStatics.GetPlayerCharacter` 0)))
  (set `self.As BP Player` _asbp_player))

(event `self.ReceiveActorBeginOverlap`
  (params (OtherActor :type "Actor Object Reference"))
  (bind _as_bp_player (`self.As BP Player`))
  (bind _cube (`self.Cube`))
  (if (== OtherActor _as_bp_player)
    (`self.K2_TeleportTo` :`self` _as_bp_player :`DestLocation` (`SceneComponent.K2_GetComponentLocation` (`self.Arrow`)))
    (`SceneComponent.SetHiddenInGame` _cube false false)
    (`PrimitiveComponent.SetCollisionEnabled` _cube "QueryAndPhysics")
    (`PrimitiveComponent.SetCollisionProfileName` _cube "BlockAll" true)
    (bind _returnvalue (`|SpawnActorFromClass` "/Game/Blueprints/CharactersLogic/BP_AI_BOSS_Baba_Yaga.BP_AI_BOSS_Baba_Yaga_C" (`KismetMathLibrary.MakeTransform` (`self.Spawn Transform Location`)) "AlwaysSpawn" "OverrideRootScale" null 200.0 "/Game/Blueprints/WeaponLogic/BP_Metla.BP_Metla_C" 200 null))
    (set `self.As_babka` _returnvalue)))

(event `Reset`
  (bind _as_babka (`self.As_babka`))
  (`SceneComponent.SetHiddenInGame` (`self.Cube`) true false)
  (`PrimitiveComponent.SetCollisionEnabled` (`self.Cube`) "NoCollision")
  (`self.K2_DestroyActor` (`/Game/Blueprints/CharactersLogic/BP_Character_Base.Current_Weapon` _as_babka))
  (`self.K2_DestroyActor` _as_babka))

(fn `UserConstructionScript`
  (`SceneComponent.K2_SetRelativeLocation` (`self.Arrow`) (`self.LocationArrow`) false false)
  (`SceneComponent.SetRelativeScale3D` (`self.Cube`) (`self.CubeScale`)))