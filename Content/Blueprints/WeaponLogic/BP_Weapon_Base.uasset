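; Base weapon actor that deals melee-style damage through a DamageBox hit volume.
; The construction script fills its stats, attack montage and icon from the DT_Weapon_Data row named by WeaponRowName.
; Attack? toggles DamageBox collision on and off.
; Overlaps send damage through BPI_Take_Damage to implementing actors other than the owner, with a shared DoOnce limiting hits to one per half second.
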(event `self.DamageBox.OnComponentBeginOverlap`
  (params (OverlappedComponent :type "PrimitiveComponent Object Reference") (OtherActor :type "Actor Object Reference") (OtherComp :type "PrimitiveComponent Object Reference") (OtherBodyIndex :type Integer) (bFromSweep :type Boolean) (SweepResult :type "HitResult Structure (by ref)"))
  (if (and (`KismetSystemLibrary.DoesImplementInterface` OtherActor "/Game/Blueprints/WeaponLogic/Interfaces/BPI_Take_Damage.BPI_Take_Damage_C") (!= OtherActor (`self.GetOwner`)))
    (`/Engine/EditorBlueprintResources/StandardMacros.DoOnce` false :!label _label
      (:`Completed`
        (message `/Game/Blueprints/WeaponLogic/Interfaces/BPI_Take_Damage.Taking_Damage` OtherActor "None" (`self.Damage`) (`self.GetOwner`))
        (`KismetSystemLibrary.Delay` 0.5)
        (goto _label :!via `Reset`)))))

(event `Attack?`
  (params (`Is_Attack?` :type Boolean))
  (bind _damagebox (`self.DamageBox`))
  (if `Is_Attack?`
    (`PrimitiveComponent.SetCollisionProfileName` _damagebox "OverlapAllDynamic" true)
    (else
      (`PrimitiveComponent.SetCollisionEnabled` _damagebox "NoCollision"))))

(fn `UserConstructionScript`
  (bind _returnvalue (`|GetDataTableRow` "/Game/Blueprints/WeaponLogic/WeaponData/DT_Weapon_Data.DT_Weapon_Data" (`self.Weapon_Row_Name`))
    (:`then`
      (bind _output_get (set `self.Weapon Data` _returnvalue))
      (bind (_weapon_name _damage _stamina_cost _wright _attribute _weapon_type _attack_montage _icon) (break `/Game/Blueprints/WeaponLogic/WeaponData/ST_Weapon_Details` _output_get))
      (set `self.Weapon Name` _weapon_name)
      (set `self.Damage` _damage)
      (set `self.Stamina Cost` _stamina_cost)
      (set `self.% Attribute` _attribute)
      (set `self.Weapon Type` _weapon_type)
      (set `self.Wright` _wright)
      (set `self.Attack Montage` _attack_montage)
      (set `self.Icon` _icon))))